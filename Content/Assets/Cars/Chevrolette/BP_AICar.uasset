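; AI-driven race car that follows the VehiclePath spline matching its track index until the race ends, then handbrakes with random steering.
; Each tick it steers toward a look-ahead spline point, scaling throttle and brake by steering amount, with randomized max throttle and steering range.
; A forward sphere trace then overrides braking based on vehicles ahead.
; BeginPlay tints the body material and binds light toggling to UDS sunrise and sunset.
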(event Custom|AI_Path
  (bind _vehiclemovementcomponent (Variables|Default|GetVehicleMovementComponent))
  (bind _returnvalue (Utilities|AIPathRotation)
    (:Is%20Valid
      (Class|ChaosVehicleMovementComponent|SetSteeringInput _vehiclemovementcomponent _returnvalue)
      (Class|ChaosVehicleMovementComponent|SetThrottleInput _vehiclemovementcomponent (* (Variables|Default|GetMaxThrottle) (Math|Float|Absolute(Float) (- (Math|Float|Absolute(Float) _returnvalue) 1.0))))
      (Class|ChaosVehicleMovementComponent|SetBrakeInput _vehiclemovementcomponent (Math|Float|Clamp(Float) (Math|Float|Absolute(Float) _returnvalue) 0.0 0.97)))))

(event Custom|LightON
  (Rendering|SetVisibility (Variables|Default|GetScene) true true))

(event Custom|LightOFF
  (Rendering|SetVisibility (Variables|Default|GetScene) false true))

(event Custom|RaceEnd
  (bind _vehiclemovementcomponent (Variables|Default|GetVehicleMovementComponent))
  (Class|ChaosVehicleMovementComponent|SetHandbrakeInput _vehiclemovementcomponent true)
  (Class|ChaosVehicleMovementComponent|SetSteeringInput _vehiclemovementcomponent (Math|Random|RandomFloatinRange -1.0 1.0))
  (Class|ChaosVehicleMovementComponent|SetThrottleInput _vehiclemovementcomponent 0.0)
  (Variables|Default|SetbRaceEnd? true))

(event EventBeginPlay
  (Utilities|FlowControl|Delay 0.2)
  (CallFunction|ChangeColor)
  (bind _returnvalue (CallFunction|GetUDS))
  (bind _output_get (Variables|Default|SetUDS _returnvalue))
  (EventDispatchers|BindEventtoSunrise _output_get (EventDispatchers|CreateEvent :!event Custom|LightOFF))
  (EventDispatchers|BindEventtoSunset _output_get (EventDispatchers|CreateEvent :!event Custom|LightON))
  (bind _outactors (Actor|GetAllActorsOfClass "/Game/Assets/Cars/Chevrolette/VehiclePath.VehiclePath_C"))
  (for _array_element _outactors
    (if (== (Variables|/Game/Assets/Cars/Chevrolette/VehiclePath.VehiclePath_C|GetIndex _array_element) (Variables|Default|GetTrackIndx))
      (Variables|Default|SetPath _array_element))))

(event Collision|EventActorBeginOverlap
  (params (OtherActor :type Actor%20Object%20Reference)))

(event EventTick
  (params (DeltaSeconds :type Float%20%28single-precision%29))
  (if (not (Variables|Default|GetbRaceEnd?))
    (CallFunction|AIPath)
    (CallFunction|Distance)))

(fn ConstructionScript)

(fn Distance
  (bind _returnvalue (Transformation|GetActorLocation))
  (bind _vehiclemovementcomponent (Variables|Default|GetVehicleMovementComponent))
  (bind (_outhit _returnvalue_2) (Collision|SphereTraceForObjects _returnvalue (+ _returnvalue (* (Math|Vector|GetForwardVector (Transformation|GetActorRotation)) 7.5e+02)) 75.0 (Utilities|Array|MakeArray "ObjectTypeQuery5") false (Utilities|Array|MakeArray self) "None"))
  (if _returnvalue_2
    (Class|ChaosVehicleMovementComponent|SetBrakeInput _vehiclemovementcomponent (Math|Float|Lerp 0.0 0.85 (Math|Float|NormalizetoRange (Math|Vector|VectorLength (/ (.Location (Collision|BreakHitResult _outhit)) (Transformation|GetActorLocation))) 0.0 7.5e+02)))
    (return)
    (else
      (Class|ChaosVehicleMovementComponent|SetBrakeInput _vehiclemovementcomponent 0.0)
      (return))))

(fn ChangeColor
  (bind _mesh (Variables|Character|GetMesh))
  (bind _returnvalue (Rendering|Material|CreateDynamicMaterialInstance _mesh 1 (Rendering|Material|GetMaterial _mesh 1) "None" :!class /Script/Engine.PrimitiveComponent))
  (Rendering|Material|SetVectorParameterValue _returnvalue "BaseColor" (Variables|Default|GetColor) :!class /Script/Engine.MaterialInstanceDynamic)
  (return))