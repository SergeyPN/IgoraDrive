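; BP_Corvette_c7 is a Corvette C7 car Blueprint whose graph controls tire dust effects.
; TireDustOn_Event activates and resets four PSmokeBikes smoke components together, and TireDustOff_Event deactivates them without a reset.
; The file shows no caller for either event, and the construction script is empty.
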(event Custom|TireDustOff_Event
  (Components|Activation|SetActive (Variables|Default|GetP_SmokeBikes1) false false))

(event Custom|TireDustOn_Event
  (Components|Activation|SetActive (Variables|Default|GetP_SmokeBikes1) true true))

(fn ConstructionScript)