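; BP_Cruiser is a car Blueprint that exposes events for switching its water splash and dust particle effects.
; WaterSplash_Event flips the wide splash component's active state on each call, while DustOn_Event and DustOff_Event explicitly activate or deactivate four smoke components together without resetting them.
; It holds no movement or trigger logic, and its construction script is empty.
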(event Custom|WaterSplash_Event
  (Components|Activation|ToggleActive (Variables|Default|GetP_WaterSplash_LargeWide)))

(event Custom|DustOff_Event
  (Components|Activation|SetActive (Variables|Default|GetP_SmokeBikes1) false false))

(event Custom|DustOn_Event
  (Components|Activation|SetActive (Variables|Default|GetP_SmokeBikes1) true false))

(fn ConstructionScript)