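; BP_1Light is a light actor that switches its spotlight with the day-night cycle of UDS, likely Ultra Dynamic Sky.
; On BeginPlay it gets and stores the UDS reference and binds events to its sunrise and sunset.
; EnableLight shows the SpotLight and calls Sunset, while DisableLight hides it and calls Sunrise.
; Tick is unused, so the light is purely event-driven.
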(event Custom|DisableLight
  (Rendering|SetVisibility (Variables|Default|GetSpotLight) false false)
  (Rendering|SetVisibility (Variables|Default|GetSpotLight) false false)
  (Default|CallSunrise))

(event Custom|EnableLight
  (Rendering|SetVisibility (Variables|Default|GetSpotLight) true false)
  (Rendering|SetVisibility (Variables|Default|GetSpotLight) true false)
  (Default|CallSunset))

(event EventBeginPlay
  (bind _returnvalue (CallFunction|GetUDS))
  (bind _output_get (Variables|Default|SetUDS _returnvalue))
  (EventDispatchers|BindEventtoSunrise _output_get (EventDispatchers|CreateEvent :!event Custom|DisableLight))
  (EventDispatchers|BindEventtoSunset _output_get (EventDispatchers|CreateEvent :!event Custom|EnableLight)))

(event Collision|EventActorBeginOverlap
  (params (OtherActor :type Actor%20Object%20Reference)))

(event EventTick
  (params (DeltaSeconds :type Float%20%28single-precision%29)))

(fn ConstructionScript)