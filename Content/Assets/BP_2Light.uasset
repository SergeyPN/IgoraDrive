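; BP_2Light is a light actor that hooks into the day-night cycle through the sky actor returned by GetUDS.
; On BeginPlay it caches that UDS reference and binds events to its sunrise and sunset notifications.
; EnableLight and DisableLight toggle the root component's visibility, propagated to all children, then call Sunset and Sunrise respectively.
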(event Custom|DisableLight
  (Rendering|SetVisibility (Variables|Default|GetDefaultSceneRoot) false true)
  (Default|CallSunrise))

(event Custom|EnableLight
  (Rendering|SetVisibility (Variables|Default|GetDefaultSceneRoot) true true)
  (Default|CallSunset))

(event EventBeginPlay
  (bind _returnvalue (CallFunction|GetUDS))
  (bind _output_get (Variables|Default|SetUDS _returnvalue))
  (EventDispatchers|BindEventtoSunrise _output_get (EventDispatchers|CreateEvent :!event Custom|DisableLight))
  (EventDispatchers|BindEventtoSunset _output_get (EventDispatchers|CreateEvent :!event Custom|EnableLight)))

(fn ConstructionScript)