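; Player camera pawn that pans, rotates and zooms by mouse via Enhanced Input and runs an idle demonstration mode.
; Spring-arm length drives curves scaling pan and zoom speed, with Tick smoothing zoom.
; A timer starts the demonstration, which focuses on tagged buildings; input stops it and eases the camera back to its saved position.
; It also switches ambient sound on sunrise and sunset; touch movement and pinch logic are mostly unwired.
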(event Custom|Night
  (Effects|Components|ParticleSystem|SetIntParameter (Variables|Default|GetAmbientSound) "State" 1))

(event Custom|Day
  (Effects|Components|ParticleSystem|SetIntParameter (Variables|Default|GetAmbientSound) "State" 0))

(event Custom|StopDemonstrationMode
  (bind _dm_switchbuildingtimer (Variables|Default|GetDM_SwitchBuildingTimer))
  (Default|CallDemonstrationEnd)
  (Utilities|Time|ClearandInvalidateTimerbyHandle (Variables|Default|GetDemonstrationTimer))
  (if (Variables|Default|GetbDemonstration?)
    (Default|ExitfromDemonstration (Variables|/Game/Blueprints/Main/MainPlayerController.MainPlayerController_C|GetMainWidget (Variables|Default|GetAs%20Main%20Player%20Controller)))
    (Variables|Default|SetbDemonstration? false)
    (Variables|Default|SetDemonstrationMode_BuildingIndex 0)
    (CallFunction|Peace self (Variables|Default|GetPeaceLocation) 1.0)
    (if (Utilities|Time|IsValidTimerHandle _dm_switchbuildingtimer)
      (Utilities|Time|ClearandInvalidateTimerbyHandle _dm_switchbuildingtimer))))

(event Custom|PlayDemonstration
  (if (not (Variables|Default|GetBuildingInteract))
    (bind _returnvalue (Utilities|Time|SetTimerbyEvent (EventDispatchers|CreateEvent :!event Custom|DemonstrationMode) (CallFunction|TimerDemonstrationCalculate)))
    (Variables|Default|SetDemonstrationTimer _returnvalue)))

(event Custom|DemonstrationMode
  (Default|CallDemonstrationStart)
  (Default|DemonstrationMode (Variables|/Game/Blueprints/Main/MainPlayerController.MainPlayerController_C|GetMainWidget (Variables|Default|GetAs%20Main%20Player%20Controller)))
  (Variables|Default|SetbDemonstration? true)
  (bind _outactors (Actor|GetAllActorswithTag "Building"))
  (if (> (Variables|Default|GetDemonstrationMode_BuildingIndex) (Utilities|Array|Length _outactors))
    (Variables|Default|SetDemonstrationMode_BuildingIndex 0))
  (Default|BuildingInteract (Actor|GetComponentbyClass (Utilities|Array|Get(acopy) _outactors (Variables|Default|GetDemonstrationMode_BuildingIndex)) "/Game/Blueprints/Components/BuildingInteractive.BuildingInteractive_C") true 0.5 true)
  (bind _returnvalue (Utilities|Time|SetTimerbyEvent (EventDispatchers|CreateEvent :!event Custom|DemonstrationMode) 15.0 true))
  (Variables|Default|SetDM_SwitchBuildingTimer _returnvalue)
  (bind _result (Math|Integer|IncrementInt (Variables|Default|GetDemonstrationMode_BuildingIndex))
    (:%20%20
      (Variables|Default|SetDemonstrationMode_BuildingIndex _result)
      (Actor|GetAllActorswithTag "Building"))))

(event EventTick
  (params (DeltaSeconds :type Float%20%28single-precision%29))
  (bind _target_arm_length_new (Variables|Default|GetTarget%20Arm%20Length%20New))
  (if (not (Math|Float|NearlyEqual(Float) (Variables|/Script/Engine.SpringArmComponent|GetTargetArmLength (Variables|Default|GetSpringArm)) _target_arm_length_new 1e+01))
    (Variables|/Script/Engine.SpringArmComponent|SetTargetArmLength (Variables|Default|GetSpringArm) (Math|Interpolation|FInterpTo (Variables|/Script/Engine.SpringArmComponent|GetTargetArmLength (Variables|Default|GetSpringArm)) _target_arm_length_new (Utilities|Time|GetWorldDeltaSeconds) (Math|Float|Lerp 3.0 1.0 (CallFunction|CameraSpringArmNormalize))))))

(event EventPeace
  (params (Location :type Vector :default "0, 0, 0") (PlayRate :type Float%20%28double-precision%29))
  (Variables|Default|SetActorLocation Location)
  (Components|Timeline|SetPlayRate (Variables|Default|GetMoveToLocationTimeline) PlayRate)
  (bind _movetoalpha (Timeline|MoveToLocationTimeline PlayFromStart)
    (:Update
      (Transformation|SetActorLocation (Math|Vector|Lerp(Vector) (Transformation|GetActorLocation) (Variables|Default|GetActorLocation) _movetoalpha) false false))))

(event EventReturnCamera
  (Game|Player|SetViewTargetwithBlend (Game|GetPlayerController 0) self 1.0 "VTBlend_Cubic" 0.5 false)
  (Variables|Default|SetInteracted? false)
  (Audio|SpawnSound2D "/Game/Assets/Sounds/Camera_Move_Cue.Camera_Move_Cue" 1.0 1.0 0.0 0)
  (Variables|Default|SetBuildingInteract false))

(event EventBeginPlay
  (bind _returnvalue (Game|GetPlayerController 0))
  (bind _returnvalue_2 (PlayerController|LocalPlayerSubsystems|GetEnhancedInputLocalPlayerSubsystem _returnvalue))
  (bind _asmain_player_controller (Utilities|Casting|CastToMainPlayerController (Game|GetPlayerController 0)))
  (Variables|Default|SetAs%20Main%20Player%20Controller _asmain_player_controller)
  (bind _asmain_game_instance (Utilities|Casting|CastToMainGameInstance (Game|GetGameInstance)))
  (Variables|Default|SetAs%20Main%20Game%20Instance _asmain_game_instance)
  (Utilities|IsValid _returnvalue_2
    (:Is%20Valid
      (Input|AddMappingContext _returnvalue_2 "/Game/Blueprints/Character/Inputs/MainInputContext.MainInputContext" 0 "(bIgnoreAllPressedKeysUntilRelease=True,bForceImmediately=False,bNotifyUserSettings=False)")
      (CallFunction|PlayDemonstration)
      (Variables|Default|SetPeaceLocation (Transformation|GetActorLocation))
      (bind _returnvalue_3 (CallFunction|GetUDS))
      (EventDispatchers|BindEventtoSunset _returnvalue_3 (delegate Custom|Night))
      (EventDispatchers|BindEventtoSunrise _returnvalue_3 (delegate Custom|Day))
      (bind _returnvalue_4 (Audio|SpawnSound2D "/Game/Assets/Sounds/Igora_AmbientSound_Cue.Igora_AmbientSound_Cue" 1.0 1.0 0.0 0))
      (Variables|Default|SetAmbientSound _returnvalue_4)
      (bind _outactors (Actor|GetAllActorsOfClass "/Game/Blueprints/Actor/MasterInteractive.MasterInteractive_C"))
      (Variables|Default|SetInteractive _outactors))))

(event Input|KeyboardEvents|AnyKey
  (params (Key :type Key%20Structure :default "None"))
  (:Pressed
    (CallFunction|StopDemonstrationMode))
  (:Released
    (CallFunction|PlayDemonstration)))

(fn ConstructionScript)

(fn GetClickDistance
  (bind _returnvalue (Game|GetPlayerController 0))
  (bind (_locationx _locationy) (Game|Player|GetMousePosition _returnvalue))
  (bind _returnvalue_2 (Math|Vector2D|MakeVector2D _locationx _locationy))
  (Variables|Default|SetCurrentMousePosition _returnvalue_2)
  (return _returnvalue_2))

(fn CameraSpringArmNormalize
  (return (Math|Float|NormalizetoRange (Variables|/Script/Engine.SpringArmComponent|GetTargetArmLength (Variables|Default|GetSpringArm)) (Variables|Default|GetArmLength%20Min) (Variables|Default|GetArmLength%20Max))))

(fn GetTouchDistance
  (bind _returnvalue (Game|GetPlayerController 0))
  (bind (_locationx _locationy) (Class|PlayerController|GetInputTouchState _returnvalue "Touch1"))
  (bind _returnvalue_2 (Math|Vector2D|MakeVector2D _locationx _locationy))
  (Variables|Touch|SetCurrentPositionTouch _returnvalue_2)
  (return _returnvalue_2))

(fn GetTouchDistanceZoom
  (bind _returnvalue (Game|GetPlayerController 0))
  (bind (_locationx _locationy) (Class|PlayerController|GetInputTouchState _returnvalue "Touch2"))
  (bind (_locationx_2 _locationy_2) (Class|PlayerController|GetInputTouchState _returnvalue "Touch1"))
  (return (Math|Vector2D|Vector2DLength (- (Math|Vector2D|MakeVector2D _locationx_2 _locationy_2) (Math|Vector2D|MakeVector2D _locationx _locationy)))))

(fn Pinch
  (params (Pinch_Value_Current1 :type Float%20%28double-precision%29))
  (LocalVariables|SetPinch_Value_Current Pinch_Value_Current1)
  (if (or (>= (select (> (LocalVariables|GetPinch_Value_Current) (Variables|Touch|GetPinchValuePrevious)) (* (- (/ (LocalVariables|GetPinch_Value_Current) (Variables|Touch|GetPinchValuePrevious)) 1.0) -1.0) (- (/ (Variables|Touch|GetPinchValuePrevious) (LocalVariables|GetPinch_Value_Current)) 1.0)) 1.0) (<= (select (> (LocalVariables|GetPinch_Value_Current) (Variables|Touch|GetPinchValuePrevious)) (* (- (/ (LocalVariables|GetPinch_Value_Current) (Variables|Touch|GetPinchValuePrevious)) 1.0) -1.0) (- (/ (Variables|Touch|GetPinchValuePrevious) (LocalVariables|GetPinch_Value_Current)) 1.0)) -1.0))
    (Variables|Touch|SetPinchValuePrevious (LocalVariables|GetPinch_Value_Current))
    (else
      (Variables|Default|SetTarget%20Arm%20Length%20New (Math|Float|Clamp(Float) (+ (* (* (Math|Float|Clamp(Float) (select (> (LocalVariables|GetPinch_Value_Current) (Variables|Touch|GetPinchValuePrevious)) (* (- (/ (LocalVariables|GetPinch_Value_Current) (Variables|Touch|GetPinchValuePrevious)) 1.0) -1.0) (- (/ (Variables|Touch|GetPinchValuePrevious) (LocalVariables|GetPinch_Value_Current)) 1.0)) -1.0) (Variables|Touch|GetPinchSpeedMultiply)) (Math|Curves|GetFloatValue (Variables|Default|GetCameraZoomCurve) (CallFunction|CameraSpringArmNormalize))) (Variables|/Script/Engine.SpringArmComponent|GetTargetArmLength (Variables|Default|GetSpringArm))) (Variables|Default|GetArmLength%20Min) (Variables|Default|GetArmLength%20Max)))
      (Variables|Touch|SetPinchValuePrevious (LocalVariables|GetPinch_Value_Current)))))

(fn TimerDemonstrationCalculate
  (return (* (Variables|Default|GetTime) (Utilities|Select :Index (Variables|/Game/Blueprints/Main/MainGameInstance.MainGameInstance_C|GetSelectedTimer (Variables|Default|GetAs%20Main%20Game%20Instance)) :Option%200 1.0 :Option%201 2.0 :Option%202 3.0 :Option%203 4.0 :Option%204 5.0 :Option%205 1e+01))))

(fn GetPeaceInfo
  (bind _returnvalue (Transformation|GetActorLocation))
  (bind _peacelocation (Variables|Default|GetPeaceLocation))
  (bind _returnvalue_2 (- _peacelocation _returnvalue))
  (bind _returnvalue_3 (Math|Vector|VectorLength _returnvalue_2))
  (return _peacelocation _returnvalue_3 (Math|Float|NormalizetoRange _returnvalue_3 0.0 3.5e+04)))

(fn InputVector
  (params (X :type Float%20%28double-precision%29) (Y :type Float%20%28double-precision%29) (Speed :type Float%20%28double-precision%29))
  (return (* (* (+ (* (Class|KismetMathLibrary|VectorNormal2D (Transformation|GetActorRightVector) 0.0001) (* X -1.0)) (* (Class|KismetMathLibrary|VectorNormal2D (Transformation|GetActorForwardVector) 0.0001) Y)) (* (Math|Curves|GetFloatValue (Variables|Default|GetCameraMoveCurve) (CallFunction|CameraSpringArmNormalize)) Speed)) -1.0)))

(fn InputRotation
  (params (Xinput :type Float%20%28double-precision%29) (Yinput :type Float%20%28double-precision%29) (Speed :type Float%20%28double-precision%29))
  (bind _returnvalue (Transformation|GetActorRotation))
  (return (Math|Float|ClampAngle (+ (* (* Yinput -1.0) Speed) (.pitch _returnvalue)) (Variables|Default|GetMin%20Angle%20Degrees) (Variables|Default|GetMax%20Angle%20Degrees)) (+ (* Xinput Speed) (.yaw _returnvalue))))

(event Input|EnhancedActionEvents|EnhancedInputActionIA_TouchMoveCamera
  (params (ActionValue :type Vector%202D%20Structure) (ElapsedSeconds :type Float%20%28double-precision%29) (TriggeredSeconds :type Float%20%28double-precision%29) (InputAction :type Input%20Action%20Object%20Reference :default "/Game/Blueprints/Character/Inputs/InputActions/IA_TouchMoveCamera.IA_TouchMoveCamera"))
  ;[0 0 0] Touch Input Action
  ;;[1 1 1] CameraMovement
)

(event Input|EnhancedActionEvents|EnhancedInputActionIA_TouchRotateCamera
  (params (ActionValue :type Vector%202D%20Structure) (ElapsedSeconds :type Float%20%28double-precision%29) (TriggeredSeconds :type Float%20%28double-precision%29) (InputAction :type Input%20Action%20Object%20Reference :default "/Game/Blueprints/Character/Inputs/InputActions/IA_TouchRotateCamera.IA_TouchRotateCamera"))
  ;[0 0 0] Touch Input Action
  ;;[1 1 1] CameraRotation
)

(event Input|EnhancedActionEvents|EnhancedInputActionIA_TouchZoomCamera
  (params (ActionValue :type Float%20%28double-precision%29) (ElapsedSeconds :type Float%20%28double-precision%29) (TriggeredSeconds :type Float%20%28double-precision%29) (InputAction :type Input%20Action%20Object%20Reference :default "/Game/Blueprints/Character/Inputs/InputActions/IA_TouchZoomCamera.IA_TouchZoomCamera"))
  ;[0 0 0] Touch Input Action
  ;;[1 1 1] CameraZoom
)

(event Input|EnhancedActionEvents|EnhancedInputActionIA_MoveMouse
  (params (ActionValue :type Boolean) (ElapsedSeconds :type Float%20%28double-precision%29) (TriggeredSeconds :type Float%20%28double-precision%29) (InputAction :type Input%20Action%20Object%20Reference :default "/Game/Blueprints/Character/Inputs/InputActions/IA_MoveMouse.IA_MoveMouse"))
  ;[0 0 0] Click Input Action
  ;;[1 1 1] ClickMovement
  (:Triggered
    (Utilities|FlowControl|Sequence
      (:then_0
        (Class|PawnMovementComponent|AddInputVector (Variables|Default|GetFloatingPawnMovement) (CallFunction|InputVector (.x (stale _returnvalue)) (.y (stale _returnvalue)) -4.0) false)
        (Variables|Default|SetPreviousMousePosition (Variables|Default|GetCurrentMousePosition)))))
  (:Started
    (bind _returnvalue (Utilities|StartClickPosition))))

(event Input|EnhancedActionEvents|EnhancedInputActionIA_RotateMouse
  (params (ActionValue :type Boolean) (ElapsedSeconds :type Float%20%28double-precision%29) (TriggeredSeconds :type Float%20%28double-precision%29) (InputAction :type Input%20Action%20Object%20Reference :default "/Game/Blueprints/Character/Inputs/InputActions/IA_RotateMouse.IA_RotateMouse"))
  ;[0 0 0] Click Input Action
  ;;[1 1 1] ClickRotation
  (:Triggered
    (Utilities|FlowControl|Sequence
      (:then_0
        (Transformation|SetActorRotation (Math|Rotator|MakeRotator 0.0 (.Y (CallFunction|InputRotation (.x (stale _returnvalue)) (.y (stale _returnvalue)) 5e+01)) (.Z (CallFunction|InputRotation (.x (stale _returnvalue)) (.y (stale _returnvalue)) 5e+01))))
        (Variables|Default|SetPreviousMousePosition (Variables|Default|GetCurrentMousePosition)))))
  (:Started
    (bind _returnvalue (Utilities|StartClickPosition))))

(event Input|EnhancedActionEvents|EnhancedInputActionIA_ZoomMouse
  (params (ActionValue :type Float%20%28double-precision%29) (ElapsedSeconds :type Float%20%28double-precision%29) (TriggeredSeconds :type Float%20%28double-precision%29) (InputAction :type Input%20Action%20Object%20Reference :default "/Game/Blueprints/Character/Inputs/InputActions/IA_ZoomMouse.IA_ZoomMouse"))
  (bind _returnvalue (CallFunction|CameraSpringArmNormalize))
  (bind _springarm (Variables|Default|GetSpringArm))
  (bind _camerazoomcurve (Variables|Default|GetCameraZoomCurve))
  (bind _returnvalue_2 (Math|Curves|GetFloatValue _camerazoomcurve _returnvalue))
  (bind _targetarmlength (Variables|/Script/Engine.SpringArmComponent|GetTargetArmLength _springarm))
  (bind _returnvalue_3 (* _returnvalue_2 9.5e+03))
  ;[0 0 0] Click Input Action
  ;;[1 1 1] MouseZoom
  (:Triggered
    (Utilities|FlowControl|Sequence
      (:then_0
        (Variables|Default|SetTarget%20Arm%20Length%20New (Math|Float|Clamp(Float) (Math|Float|SelectFloat (+ _targetarmlength _returnvalue_3) (- _targetarmlength _returnvalue_3) (< (Variables|Default|GetZoom%20Action%20Value) 0.0)) (Variables|Default|GetArmLength%20Min) (Variables|Default|GetArmLength%20Max))))))
  (:Started
    (Variables|Default|SetZoom%20Action%20Value ActionValue)))

(event Input|KeyboardEvents|1
  (params (Key :type Key%20Structure :default "None"))
  (bind _interactive (Variables|Default|GetInteractive))
  (:Pressed
    (bind _returnvalue (Actor|GetActorOfClass "/Game/Blueprints/Actor/MainRaceInteraction.MainRaceInteraction_C"))
    (Utilities|IsValid (Utilities|Array|Get(acopy) _interactive (Utilities|Array|FindItem _interactive _returnvalue))
      (:Is%20Valid
        (Default|EnableEvent (Utilities|Array|Get(acopy) _interactive (Utilities|Array|FindItem _interactive _returnvalue)))))))

(event Input|KeyboardEvents|2
  (params (Key :type Key%20Structure :default "None")))

(event Input|KeyboardEvents|3
  (params (Key :type Key%20Structure :default "None")))

(event Input|KeyboardEvents|4
  (params (Key :type Key%20Structure :default "None")))

(event Input|TouchEvents|InputTouch
  (params (Location :type Vector) (FingerIndex :type ETouchIndex%20Enum))
  (:Pressed
    (Variables|Default|SetTouch true)
    (CallFunction|StopDemonstrationMode)
    (if (not (Variables|Default|GetTouchInterface))
      (Utilities|FlowControl|Delay 0.2)
      (switch Utilities|FlowControl|Switch|SwitchonETouchIndex FingerIndex
        (:Touch1
          (Utilities|TouchBranch "NewEnumerator1" "NewEnumerator3"
            (:true
              (Variables|Default|SetFinger%20Index "Touch1")
              (Variables|Default|SetTouchStateEnum "NewEnumerator2"))))
        (:Touch2
          (Utilities|TouchBranch "NewEnumerator2" "NewEnumerator3"
            (:true
              (Variables|Default|SetFinger%20Index "Touch2")
              (Variables|Default|SetTouchStateEnum "NewEnumerator1"))))
        (:Touch3
          (Utilities|TouchBranch "NewEnumerator2" "NewEnumerator1"
            (:true
              (Variables|Default|SetFinger%20Index "Touch3")
              (Variables|Default|SetTouchStateEnum "NewEnumerator3")))))
      (else
        (Variables|Default|SetLocation Location :!label _label))))
  (:Released
    (Utilities|FlowControl|Delay 0.2)
    (Variables|Default|SetTouch false)
    (Variables|Default|SetTouchStateEnum "NewEnumerator0")
    (CallFunction|PlayDemonstration))
  (:Moved
    (goto _label)))