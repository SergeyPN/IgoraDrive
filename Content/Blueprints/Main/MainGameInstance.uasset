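; Game instance that prepares building and track content at startup, tracks loading progress and opens the "drive" level.
; Init applies the sound setting, then either loads BP_Save or fetches a remote JSON catalogue through VaRest.
; Counter macros and completion callbacks walk buildings and nested tracks sequentially, downloading missing photos and videos, plus QR codes, into Content/Movies.
; The resulting info and local paths fill struct arrays that are saved for later launches.
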(event Custom|GetRequests
  (params (Request :type Va%20Rest%20Request%20JSON%20Object%20Reference))
  (Variables|JSON|SetRequest Request)
  (bind _output_get (Variables|JSON|SetDataField (Class|VaRestJsonObject|GetArrayField (Class|VaRestRequestJSON|GetResponseObject (Variables|JSON|GetRequest)) "Data")))
  (Variables|JSON|SetMaxDataField (Utilities|Array|Length _output_get))
  (bind _returnvalue (Class|VaRestJsonValue|AsObject (Utilities|Array|Get(acopy) (Variables|JSON|GetDataField) (Variables|Building|GetMainIndex))))
  (CallFunction|GetBuildingInfo _returnvalue)
  (Variables|Track|SetTrackField (Class|VaRestJsonObject|GetArrayField _returnvalue "tracks"))
  (Variables|Track|SetMaxTrackField (Utilities|Array|Length (Variables|Track|GetTrackField))))

(event Custom|UPD_Data
  ;[1 1 1] Upd
  (Variables|Save|SetLoading 0.0)
  (Variables|Building|SetMainIndex 0)
  (Utilities|Array|Clear (Variables|Building|GetSoftMainPhotosImage))
  (Utilities|Array|Clear (Variables|Track|GetSoftTrackPhotosImage))
  (Utilities|Array|Clear (Variables|Building|GetBuildingStructure))
  (Utilities|Array|Clear (Variables|Building|GetVideoURLs))
  (Utilities|Array|Clear (Variables|Building|GetPhotosURLs))
  (Utilities|Array|Clear (Variables|Track|GetTrackPhotosURLs))
  (Utilities|Array|Clear (Variables|Track|GetTrackVideoURLs))
  (Utilities|Array|Clear (Variables|Track|GetTracksStructure))
  (CallFunction|ConstructJSONobj (delegate Custom|GetRequests)))

(event Custom|SuccessDownloadTrack
  (|TackJsonInfo_2_2)
  (Utilities|FlowControl|Delay 0.2)
  (CallFunction|NextTrack))

(event Custom|SuccessDownloadBuilding
  (|BuildingJsonInfo)
  (Utilities|FlowControl|Delay 0.2)
  (CallFunction|NextIndex))

(event Custom|ProgressVideoBuilding
  (params (BytesReceived :type Integer64) (ContentLength :type Integer64) (ProgressRatio :type Float%20%28single-precision%29))
  (Variables|Save|SetLoading ProgressRatio))

(event Custom|ProgressPhotoBuild
  (params (BytesReceived :type Integer64) (ContentLength :type Integer64) (ProgressRatio :type Float%20%28single-precision%29))
  (Variables|Save|SetLoading ProgressRatio))

(event Custom|DownloadImageSuccess
  (params (Result :type EDownloadToStorageResult%20Enum :default "Success"))
  (Utilities|CheckSuccessDownloadedImage :!label _label
    (:true
      (CallFunction|ImportImage (Variables|Building|GetMainPhotos) (Variables|Building|GetPhotosURLs))
      (CallFunction|BuildingDownloadVideos))
    (:false
      (bind _returnvalue (CallFunction|DownloadContents (Utilities|Array|Get(acopy) (Variables|Building|GetMainPhotos) (Variables|Default|GetBuildingPhotos)) (delegate Custom|ProgressPhotoBuild) (delegate Custom|DownloadImageSuccess)))
      (if _returnvalue
        (goto _label)))))

(event Custom|BuildingDownloadVideos
  (bind _mainvideos (Variables|Building|GetMainVideos))
  (if (Utilities|Array|IsEmpty _mainvideos)
    (CallFunction|SuccessDownloadBuilding)
    (else
      (Variables|Default|SetBuildingMaxVideos (Utilities|Array|Length _mainvideos))
      (bind _returnvalue (CallFunction|DownloadContents (Utilities|Array|Get(acopy) _mainvideos (Variables|Default|GetBuildingVideos)) (delegate Custom|ProgressVideoBuilding) (delegate Custom|DownloadVideoSuccess) :!label _label))
      (if _returnvalue
        (Utilities|CheckSuccessDownloadedVideo
          (:true
            (CallFunction|GetVideosPath (Variables|Building|GetVideoURLs) (Variables|Building|GetMainVideos))
            (CallFunction|SuccessDownloadBuilding))
          (:false
            (goto _label)))))))

(event Custom|DownloadVideoSuccess
  (params (Result :type EDownloadToStorageResult%20Enum :default "Success"))
  (Utilities|CheckSuccessDownloadedVideo :!label _label
    (:true
      (CallFunction|GetVideosPath (Variables|Building|GetVideoURLs) (Variables|Building|GetMainVideos))
      (CallFunction|SuccessDownloadBuilding))
    (:false
      (bind _returnvalue (CallFunction|DownloadContents (Utilities|Array|Get(acopy) (Variables|Building|GetMainVideos) (Variables|Default|GetBuildingVideos)) (delegate Custom|ProgressVideoBuilding) (delegate Custom|DownloadVideoSuccess)))
      (if _returnvalue
        (goto _label)))))

(event Custom|ProgressPhotoTrack
  (params (BytesReceived :type Integer64) (ContentLength :type Integer64) (ProgressRatio :type Float%20%28single-precision%29))
  (Variables|Save|SetLoading ProgressRatio))

(event Custom|GetBuildingInfo
  (params (JsonObject :type Va%20Rest%20Json%20Object%20Object%20Reference))
  (bind _mainphotos (Variables|Building|GetMainPhotos))
  (Variables|JSON|SetMainJsonObject JsonObject)
  (Utilities|Array|Clear (Variables|Building|GetMainPhotos))
  (Utilities|Array|Clear (Variables|Building|GetMainVideos))
  (Utilities|Array|Clear (Variables|Building|GetVideoURLs))
  (Utilities|Array|Clear (Variables|Building|GetPhotosURLs))
  (Variables|Default|SetBuildingPhotos 0)
  (Variables|Default|SetBuildingMaxVideos 0)
  (CallFunction|GetURLs (Variables|Building|GetMainPhotos) (Variables|JSON|GetMainJsonObject) "photos" "Path")
  (CallFunction|GetURLs (Variables|Building|GetMainVideos) (Variables|JSON|GetMainJsonObject) "videos" "Path")
  (Utilities|FlowControl|Delay 0.2)
  (if (Utilities|Array|IsEmpty _mainphotos)
    (CallFunction|BuildingDownloadVideos)
    (else
      (Variables|Default|SetBuildingMaxPhotos (Utilities|Array|Length _mainphotos))
      (bind _returnvalue (CallFunction|DownloadContents (Utilities|Array|Get(acopy) _mainphotos (Variables|Default|GetBuildingPhotos)) (delegate Custom|ProgressPhotoBuild) (delegate Custom|DownloadImageSuccess) :!label _label))
      (if _returnvalue
        (Utilities|CheckSuccessDownloadedImage
          (:true
            (CallFunction|ImportImage (Variables|Building|GetMainPhotos) (Variables|Building|GetPhotosURLs))
            (CallFunction|BuildingDownloadVideos))
          (:false
            (goto _label)))))))

(event Custom|ProgressVideoTrack
  (params (BytesReceived :type Integer64) (ContentLength :type Integer64) (ProgressRatio :type Float%20%28single-precision%29))
  (Variables|Save|SetLoading ProgressRatio))

(event Custom|TrackDownloadVideos
  (bind _trackvideosstracture (Variables|Track|GetTrackVideosStracture))
  (Variables|Default|SetTrackVideos 0)
  (if (Utilities|Array|IsEmpty _trackvideosstracture)
    (CallFunction|SuccessDownloadTrack)
    (else
      (Variables|Default|SetTrackMaxVideos (Utilities|Array|Length _trackvideosstracture))
      (bind _returnvalue (CallFunction|DownloadContents (Utilities|Array|Get(acopy) _trackvideosstracture (Variables|Default|GetTrackVideos)) (delegate Custom|ProgressVideoTrack) (delegate Custom|SuccessTrackDownloadVideos) :!label _label))
      (if _returnvalue
        (Utilities|CheckSuccessDownloadedVideoTrack
          (:true
            (CallFunction|GetVideosPath (Variables|Track|GetTrackVideoURLs) (Variables|Track|GetTrackVideosStracture))
            (CallFunction|SuccessDownloadTrack))
          (:false
            (goto _label)))))))

(event Custom|SuccessTrackDownloadImage
  (params (Result :type EDownloadToStorageResult%20Enum :default "Success"))
  (Utilities|CheckSuccessDownloadedImageTrack :!label _label
    (:true
      (CallFunction|ImportImage (Variables|Track|GetTrackPhotosStracture) (Variables|Track|GetTrackPhotosURLs))
      (CallFunction|TrackDownloadVideos))
    (:false
      (bind _returnvalue (CallFunction|DownloadContents (Utilities|Array|Get(acopy) (Variables|Track|GetTrackPhotosStracture) (Variables|Default|GetTrackPhotos)) (delegate Custom|ProgressPhotoTrack) (delegate Custom|SuccessTrackDownloadImage)))
      (if _returnvalue
        (goto _label)))))

(event Custom|SuccessTrackDownloadVideos
  (params (Result :type EDownloadToStorageResult%20Enum :default "Success"))
  (Utilities|CheckSuccessDownloadedVideoTrack :!label _label
    (:true
      (CallFunction|GetVideosPath (Variables|Track|GetTrackVideoURLs) (Variables|Track|GetTrackVideosStracture))
      (CallFunction|SuccessDownloadTrack))
    (:false
      (bind _returnvalue (CallFunction|DownloadContents (Utilities|Array|Get(acopy) (Variables|Track|GetTrackVideosStracture) (Variables|Default|GetTrackVideos)) (delegate Custom|ProgressVideoTrack) (delegate Custom|SuccessTrackDownloadVideos)))
      (if _returnvalue
        (goto _label)))))

(event Custom|NextIndex
  (Utilities|CheckIndex
    (:FullCompile
      (Utilities|Array|Clear (Variables|Building|GetMainPhotosImage))
      (Utilities|Array|Clear (Variables|Track|GetHardTrackPhotosImage))
      (CallFunction|SaveGame)
      (Variables|Save|SetLoading (+ (Variables|Save|GetLoading) 0.1))
      (Utilities|FlowControl|Delay 0.2)
      (Game|OpenLevel(byName) "drive"))
    (:Loading
      (bind _returnvalue (Class|VaRestJsonValue|AsObject (Utilities|Array|Get(acopy) (Variables|JSON|GetDataField) (Variables|Building|GetMainIndex))))
      (CallFunction|GetBuildingInfo _returnvalue)
      (Variables|Track|SetTrackField (Class|VaRestJsonObject|GetArrayField _returnvalue "tracks"))
      (Variables|Track|SetMaxTrackField (Utilities|Array|Length (Variables|Track|GetTrackField))))
    (:WaitCompile
      (bind _returnvalue_2 (Class|VaRestJsonValue|AsObject (Utilities|Array|Get(acopy) (Variables|Track|GetTrackField) (Variables|Track|GetTrackIndex))))
      (Variables|Track|SetTrackJsonObject _returnvalue_2)
      (CallFunction|GetTrackInformation))))

(event Custom|FastLoading
  (CallFunction|ConstructJSONobj (delegate Custom|FastGetInfo)))

(event Custom|LoadingSavedGame
  (bind _output_get (Variables|Save|SetLoading (+ (Variables|Save|GetLoading) 0.1)))
  (if (>= _output_get 0.9)
    (Utilities|Time|ClearandInvalidateTimerbyHandle (Variables|Save|GetLoadingTimer))
    (Game|OpenLevel(byName) "drive")))

(event Custom|NextTrack
  (Utilities|CheckTrackIndex
    (:FullTrack
      (Utilities|FlowControl|Delay 0.2)
      (Variables|Track|SetTrackIndex 0)
      (CallFunction|NextIndex))
    (:Loading
      (bind _returnvalue (Class|VaRestJsonValue|AsObject (Utilities|Array|Get(acopy) (Variables|Track|GetTrackField) (Variables|Track|GetTrackIndex))))
      (Variables|Track|SetTrackJsonObject _returnvalue)
      (CallFunction|GetTrackInformation))))

(event Custom|FastGetInfo
  (params (Request :type Va%20Rest%20Request%20JSON%20Object%20Reference))
  (Variables|JSON|SetRequest Request)
  (Variables|JSON|SetDataField (Class|VaRestJsonObject|GetArrayField (Class|VaRestRequestJSON|GetResponseObject (Variables|JSON|GetRequest)) "Data")))

(event Custom|GetTrackInformation
  (bind _trackjsonobject (Variables|Track|GetTrackJsonObject))
  (bind _trackphotosstracture (Variables|Track|GetTrackPhotosStracture))
  (Utilities|Array|Clear (Variables|Track|GetTrackPhotosStracture))
  (Utilities|Array|Clear (Variables|Track|GetTrackVideosStracture))
  (Utilities|Array|Clear (Variables|Track|GetTrackPhotosURLs))
  (Utilities|Array|Clear (Variables|Track|GetTrackVideoURLs))
  (Variables|Default|SetTrackPhotos 0)
  (Variables|Default|SetTrackVideos 0)
  (CallFunction|GetURLs (Variables|Track|GetTrackPhotosStracture) _trackjsonobject "photos" "Path")
  (CallFunction|GetURLs (Variables|Track|GetTrackVideosStracture) _trackjsonobject "videos" "Path")
  (if (Utilities|Array|IsEmpty _trackphotosstracture)
    (CallFunction|TrackDownloadVideos)
    (else
      (Variables|Default|SetTrackMaxPhotos (Utilities|Array|Length _trackphotosstracture))
      (bind _returnvalue (CallFunction|DownloadContents (Utilities|Array|Get(acopy) _trackphotosstracture (Variables|Default|GetTrackPhotos)) (delegate Custom|ProgressPhotoTrack) (delegate Custom|SuccessTrackDownloadImage) :!label _label))
      (if _returnvalue
        (Utilities|CheckSuccessDownloadedImageTrack
          (:true
            (CallFunction|ImportImage (Variables|Track|GetTrackPhotosStracture) (Variables|Track|GetTrackPhotosURLs))
            (CallFunction|TrackDownloadVideos))
          (:false
            (goto _label)))))))

(event EventInit
  (CallFunction|MuteAllSound)
  (bind _returnvalue (SaveGame|DoesSaveGameExist (Variables|Save|GetSlot%20Name)))
  (if _returnvalue
    (CallFunction|LoadGame)
    (bind _returnvalue_2 (Utilities|Time|SetTimerbyEvent (delegate Custom|LoadingSavedGame) 0.35 true))
    (Variables|Save|SetLoadingTimer _returnvalue_2)
    (else
      (CallFunction|UPDData))))

(fn ConstructJSONobj
  (params (Callback :type Delegate%20%28by%20ref%29))
  (bind _returnvalue (|VaRestSubsystem))
  (bind _returnvalue_2 (Class|VaRestSubsystem|ConstructVaRestJsonObject _returnvalue))
  (Class|VaRestSubsystem|CallURL _returnvalue "https://igora.4app.pro/static/uploads/data.json" "GET" "x_www_form_urlencoded_url" _returnvalue_2 Callback)
  (return))

(fn GetURLs
  (params (Array :type Array%20of%20Media%20Structure%20Structures) (Object :type Va%20Rest%20Json%20Object%20Object%20Reference) (ArrayName :type String) (FieldName :type String))
  (for _array_element (Class|VaRestJsonObject|GetArrayField Object ArrayName)
    (bind _returnvalue (Class|VaRestJsonValue|AsObject _array_element))
    (Utilities|Array|Add Array (Utilities|Struct|MakeMediaStructure (Class|VaRestJsonObject|GetStringField _returnvalue "title") (Class|VaRestJsonObject|GetStringField _returnvalue FieldName))))
  (return))

(fn MuteAllSound
  (Class|GameplayStatics|SetBaseSoundMix (select (Variables|Save|GetbSoundOn?) "/Game/Assets/Sounds/Classes/UnMute.UnMute" "/Game/Assets/Sounds/Classes/Mute.Mute"))
  (return))

(fn GetCurrentInd)

(fn SaveGame
  (bind _buildingstructure (Variables|Building|GetBuildingStructure))
  (bind _tracksstructure (Variables|Track|GetTracksStructure))
  (bind _slot_name (Variables|Save|GetSlot%20Name))
  (bind _returnvalue (SaveGame|DoesSaveGameExist (Variables|Save|GetSlot%20Name)))
  (if _returnvalue
    (bind _returnvalue_2 (SaveGame|LoadGamefromSlot (Variables|Save|GetSlot%20Name)))
    (bind _asbp_save (Utilities|Casting|CastToBP_Save _returnvalue_2))
    (Variables|/Game/Blueprints/Main/BP_Save.BP_Save_C|SetBuildingStracture _asbp_save _buildingstructure)
    (Variables|/Game/Blueprints/Main/BP_Save.BP_Save_C|SetTrackStructure _asbp_save _tracksstructure)
    (SaveGame|SaveGametoSlot _asbp_save _slot_name)
    (else
      (bind _returnvalue_3 (SaveGame|CreateSaveGameObject "/Game/Blueprints/Main/BP_Save.BP_Save_C"))
      (Variables|/Game/Blueprints/Main/BP_Save.BP_Save_C|SetBuildingStracture _returnvalue_3 _buildingstructure)
      (Variables|/Game/Blueprints/Main/BP_Save.BP_Save_C|SetTrackStructure _returnvalue_3 _tracksstructure)
      (SaveGame|SaveGametoSlot _returnvalue_3 _slot_name)))
  (return))

(fn LoadGame
  (bind _returnvalue (SaveGame|LoadGamefromSlot (Variables|Save|GetSlot%20Name)))
  (bind _asbp_save (Utilities|Casting|CastToBP_Save _returnvalue))
  (Variables|Building|SetBuildingStructure (Variables|/Game/Blueprints/Main/BP_Save.BP_Save_C|GetBuildingStracture _asbp_save))
  (Variables|Track|SetTracksStructure (Variables|/Game/Blueprints/Main/BP_Save.BP_Save_C|GetTrackStructure _asbp_save))
  (return))

(fn DownloadContents
  (params (Structure :type Media%20Structure%20Structure) (OnProgress :type Delegate%20%28by%20ref%29) (OnComplete :type Delegate%20%28by%20ref%29))
  (bind (_filename _url) (Utilities|Struct|BreakMediaStructure Structure))
  (bind _returnvalue (Class|KismetSystemLibrary|GetProjectContentDirectory))
  (bind _returnvalue_2 (Utilities|String|Append _returnvalue "Movies/" _filename))
  (bind _output_get (Variables|Default|SetDownloadFile _returnvalue_2))
  (bind _returnvalue_3 (Class|BaseFilesDownloader|IsFileExist _output_get))
  (if _returnvalue_3
    _
    (else
      (Class|FiletoStorageDownloader|DownloadFiletoStorage _url _returnvalue_2 0.0 "" true OnProgress OnComplete)))
  (return _returnvalue_3))

(fn ImportImage
  (params (Array :type Array%20of%20Media%20Structure%20Structures) (Photos :type Array%20of%20Strings))
  (for _array_element Array
    (Utilities|Array|Add Photos (Utilities|String|Append (Class|KismetSystemLibrary|GetProjectContentDirectory) "/Movies/" (.FileName (Utilities|Struct|BreakMediaStructure _array_element)))))
  (return))

(fn GetVideosPath
  (params (TargetArray :type Array%20of%20Strings) (Array :type Array%20of%20Media%20Structure%20Structures))
  (for _array_element Array
    (Utilities|Array|Add TargetArray (Utilities|String|Append (Class|KismetSystemLibrary|GetProjectContentDirectory) "/Movies/" (.FileName (Utilities|Struct|BreakMediaStructure _array_element)))))
  (return))

(event Custom|CustomEvent
  (params (BytesReceived :type Integer64) (ContentLength :type Integer64) (ProgressRatio :type Float%20%28single-precision%29)))

(event Custom|CustomEvent_0
  (params (Result :type EDownloadToStorageResult%20Enum :default "Success"))
  (bind _mainjsonobject (Variables|JSON|GetMainJsonObject))
  (bind _returnvalue (Class|VaRestJsonObject|GetIntegerField _mainjsonobject "id"))
  (bind _returnvalue_2 (Utilities|String|ToString(Integer) _returnvalue))
  ;[1 1 1] SetupMainInformation
  (Utilities|Array|Add (Variables|Building|GetBuildingStructure) (Utilities|Struct|MakeStructure_ObjectsData _returnvalue (Class|VaRestJsonObject|GetStringField _mainjsonobject "title") (Class|VaRestJsonObject|GetStringArrayField _mainjsonobject "description") (Class|VaRestJsonObject|GetStringArrayField _mainjsonobject "services") (Class|VaRestJsonObject|GetStringArrayField _mainjsonobject "disciplines") (Utilities|String|Append "/Game" "/Movies/" "QR" _returnvalue_2 ".QR" _returnvalue_2) (Variables|Building|GetPhotosURLs) (Variables|Building|GetVideoURLs)))
  (return))

(event Custom|CustomEvent_1
  (params (BytesReceived :type Integer64) (ContentLength :type Integer64) (ProgressRatio :type Float%20%28single-precision%29)))

(event Custom|CustomEvent_2
  (params (Result :type EDownloadToStorageResult%20Enum :default "Success"))
  (bind _trackjsonobject (Variables|Track|GetTrackJsonObject))
  (bind _returnvalue (Class|VaRestJsonObject|GetIntegerField _trackjsonobject "id"))
  (bind _returnvalue_2 (Utilities|String|ToString(Integer) _returnvalue))
  (Utilities|Array|Add (Variables|Track|GetTracksStructure) (Utilities|Struct|MakeStructure_Tracks _returnvalue (Class|VaRestJsonObject|GetStringField _trackjsonobject "title") (Class|VaRestJsonObject|GetStringArrayField _trackjsonobject "description") (Class|VaRestJsonObject|GetStringArrayField _trackjsonobject "services") (Class|VaRestJsonObject|GetStringArrayField _trackjsonobject "disciplines") (Utilities|String|Append "/Game" "/Movies/" "TQR" _returnvalue_2 ".TQR" _returnvalue_2) (Class|VaRestJsonObject|GetIntegerField _trackjsonobject "center_id") (Variables|Track|GetTrackPhotosURLs) (Variables|Track|GetTrackVideoURLs) (Class|VaRestJsonObject|GetStringArrayField _trackjsonobject "covering")))
  (return))