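; Component for lamp props that adds a light to its owner and switches the mesh's material between night and day looks.
; On BeginPlay it spawns BP_2Light or BP_1Light, chosen by B2Lamp, at the static mesh's "Light" socket and binds to its sunset and sunrise events.
; SunSet and SunRise each create a dynamic instance of material slot 1 and toggle its NightDistance parameter.
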(event Custom|SunSet
  (bind _returnvalue (Components|GetOwner))
  (bind _returnvalue_2 (Actor|GetComponentbyClass _returnvalue "/Script/Engine.StaticMeshComponent"))
  (bind _returnvalue_3 (Rendering|Material|GetMaterial _returnvalue_2 1))
  (Utilities|IsValid _returnvalue_3
    (:Is%20Valid
      (bind _returnvalue_4 (Rendering|Material|CreateDynamicMaterialInstance _returnvalue_2 1 _returnvalue_3 "None" :!class /Script/Engine.PrimitiveComponent))
      (Rendering|Material|SetScalarParameterValue _returnvalue_4 "NightDistance" 1.0 :!class /Script/Engine.MaterialInstanceDynamic))))

(event Custom|SunRise
  (bind _returnvalue (Components|GetOwner))
  (bind _returnvalue_2 (Actor|GetComponentbyClass _returnvalue "/Script/Engine.StaticMeshComponent"))
  (bind _returnvalue_3 (Rendering|Material|GetMaterial _returnvalue_2 1))
  (Utilities|IsValid _returnvalue_3
    (:Is%20Valid
      (bind _returnvalue_4 (Rendering|Material|CreateDynamicMaterialInstance _returnvalue_2 1 _returnvalue_3 "None" :!class /Script/Engine.PrimitiveComponent))
      (Rendering|Material|SetScalarParameterValue _returnvalue_4 "NightDistance" 0.0 :!class /Script/Engine.MaterialInstanceDynamic))))

(event EventBeginPlay
  (bind _returnvalue (Components|GetOwner))
  (bind _returnvalue_2 (Actor|GetComponentbyClass _returnvalue "/Script/Engine.StaticMeshComponent"))
  (bind _returnvalue_3 (Transformation|GetSocketLocation _returnvalue_2 "Light"))
  (if (Variables|Default|Getb2Lamp?)
    (bind _returnvalue_4 (Game|SpawnActorfromClass "/Game/Assets/BP_2Light.BP_2Light_C" (Math|Transform|MakeTransform _returnvalue_3 "0, 0, 0" "1.000000,1.000000,1.000000") "Undefined" "MultiplyWithRoot" 0 0))
    (EventDispatchers|BindEventtoSunset _returnvalue_4 (EventDispatchers|CreateEvent :!event Custom|SunSet))
    (EventDispatchers|BindEventtoSunrise _returnvalue_4 (EventDispatchers|CreateEvent :!event Custom|SunRise))
    (else
      (bind _returnvalue_5 (Game|SpawnActorfromClass "/Game/Assets/BP_1Light.BP_1Light_C" (Math|Transform|MakeTransform _returnvalue_3 "0, 0, 0" "1.000000,1.000000,1.000000") "Undefined" "MultiplyWithRoot" 0 0))
      (EventDispatchers|BindEventtoSunset _returnvalue_5 (EventDispatchers|CreateEvent :!event Custom|SunSet))
      (EventDispatchers|BindEventtoSunrise _returnvalue_5 (EventDispatchers|CreateEvent :!event Custom|SunRise)))))