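; Actor component that makes a building selectable by click, touch or a floating screen-space name button.
; It spawns the button widget on BeginPlay, and Tick shows it only when the camera is distant.
; Selection moves the view to the building's camera spot, optionally with fades, and notifies the main widget by building ID.
; BuildingInteraction toggles button visibility and click/touch response.
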(event Custom|CustomEvent
  (params (TouchedActor :type Actor%20Object%20Reference) (ButtonPressed :type Key%20Structure :default "None"))
  (bind _playercharacter (Variables|Default|GetPlayerCharacter))
  (Variables|Default|SetTouched%20Actor TouchedActor)
  (Variables|Default|SetbFade? false)
  (if (not (Variables|Default|GetDisableButton))
    (Variables|Default|SetbFade? false)
    (Variables|Default|SetCameraSwitchSpeed 1.0)
    (Variables|Default|SetDisable%20Border? false)
    (Utilities|FlowControl|Delay 0.2)
    (if (not (Variables|/Game/Blueprints/Character/PlayerCamera.PlayerCamera_C|GetTouch _playercharacter))
      (if (not (Variables|/Game/Blueprints/Character/PlayerCamera.PlayerCamera_C|GetInteracted? _playercharacter))
        (CallFunction|CameratoActionSpots)
        (Variables|/Game/Blueprints/Character/PlayerCamera.PlayerCamera_C|SetInteracted? _playercharacter true)
        (Class|InterfaceActionInteractivewithActor|GetBuildingbyID(Message) (Variables|/Game/Blueprints/Main/MainPlayerController.MainPlayerController_C|GetMainWidget (.AsMain%20Player%20Controller (Utilities|Casting|CastToMainPlayerController (Game|GetPlayerController 0)))) (Variables|Default|GetIndex) (Variables|Default|GetDisable%20Border?) (Components|GetOwner))
        (if (not (Variables|Default|GetbFade?))
          (Default|StopDemonstrationMode (Variables|Default|GetPlayerCharacter)))))))

(event Custom|BuildingInteract
  (params (Fade? :type Boolean) (CameraSpeed :type Float%20%28double-precision%29) (SelecterdBorder? :type Boolean))
  (CallFunction|SelectBuilding self Fade? CameraSpeed SelecterdBorder?))

(event Custom|OnTouched
  (params (FingerIndex :type ETouchIndex%20Enum :default "Touch1") (TouchedActor :type Actor%20Object%20Reference))
  (bind _playercharacter (Variables|Default|GetPlayerCharacter))
  (Variables|Default|SetTouched%20Actor TouchedActor)
  (if (not (Variables|Default|GetDisableButton))
    (Variables|Default|SetbFade? false)
    (Variables|Default|SetCameraSwitchSpeed 1.0)
    (Variables|Default|SetDisable%20Border? false)
    (Utilities|FlowControl|Delay 0.2)
    (if (not (Variables|/Game/Blueprints/Character/PlayerCamera.PlayerCamera_C|GetTouch _playercharacter))
      (if (not (Variables|/Game/Blueprints/Character/PlayerCamera.PlayerCamera_C|GetInteracted? _playercharacter))
        (CallFunction|CameratoActionSpots)
        (Variables|/Game/Blueprints/Character/PlayerCamera.PlayerCamera_C|SetInteracted? _playercharacter true)
        (Class|InterfaceActionInteractivewithActor|GetBuildingbyID(Message) (Variables|/Game/Blueprints/Main/MainPlayerController.MainPlayerController_C|GetMainWidget (.AsMain%20Player%20Controller (Utilities|Casting|CastToMainPlayerController (Game|GetPlayerController 0)))) (Variables|Default|GetIndex) (Variables|Default|GetDisable%20Border?) (Components|GetOwner))
        (if (not (Variables|Default|GetbFade?))
          (Default|StopDemonstrationMode (Variables|Default|GetPlayerCharacter)))))))

(event Custom|CameraToActionSpots
  (bind _returnvalue (Game|GetPlayerController 0))
  (bind _playercameramanager (Variables|/Script/Engine.PlayerController|GetPlayerCameraManager _returnvalue))
  (if (Variables|Default|GetbFade?)
    (CameraFades|StartCameraFade :self _playercameramanager :ToAlpha 1.0 :Duration 0.5 :bHoldWhenFinished true)
    (Utilities|FlowControl|Delay 0.6)
    (if (Variables|/Game/Blueprints/Character/PlayerCamera.PlayerCamera_C|GetbDemonstration? (Variables|Default|GetPlayerCharacter))
      (Game|Player|SetViewTargetwithBlend _returnvalue (Utilities|Array|Get(acopy) (Variables|Default|GetCamera) (Variables|Default|GetCameraSpots)) (Variables|Default|GetCameraSwitchSpeed) "VTBlend_Cubic" 0.5 false)
      (Utilities|FlowControl|Delay (Variables|Default|GetCameraSwitchSpeed)))
    (CameraFades|StartCameraFade :self _playercameramanager :FromAlpha 1.0 :Duration 0.5 :bHoldWhenFinished true)
    (else
      (Game|Player|SetViewTargetwithBlend _returnvalue (Utilities|Array|Get(acopy) (Variables|Default|GetCamera) (Variables|Default|GetCameraSpots)) (Variables|Default|GetCameraSwitchSpeed) "VTBlend_Cubic" 0.5 false))))

(event EventBeginPlay
  (bind _returnvalue (Components|GetOwner))
  (bind _returnvalue_2 (Components|GetOwner))
  (bind _locationwidget (Variables|Default|GetLocationWidget))
  (bind _returnvalue_3 (Transformation|GetActorLocation _returnvalue_2))
  (bind _returnvalue_4 (+ _returnvalue_3 _locationwidget))
  (bind (_x _y _z) (Math|Vector|BreakVector _returnvalue_4))
  (EventDispatchers|BindEventtoOnInputTouchEnd _returnvalue (EventDispatchers|CreateEvent :!event Custom|OnTouched))
  (EventDispatchers|BindEventtoOnClicked _returnvalue (delegate Custom|CustomEvent))
  (bind _outactors (Actor|GetAllActorsOfClass "/Game/Blueprints/Character/PlayerCamera.PlayerCamera_C"))
  (Variables|Default|SetPlayerCharacter (Utilities|Array|Get(acopy) _outactors))
  (Utilities|FlowControl|Delay 0.5)
  (bind _returnvalue_5 (Game|AddComponentbyClass _returnvalue "/Script/UMG.WidgetComponent" true (Math|Transform|MakeTransform (Math|Vector|MakeVector _x _y (+ _z (Variables|Default|GetZ_Offset))) "0, 0, 0" "1.000000,1.000000,1.000000")))
  (bind _returnvalue_6 (UserInterface|CreateWidget "/Game/Blueprints/Widgets/BuildingNameButton.BuildingNameButton_C" (Game|GetPlayerController 0) (Variables|Default|GetIndex)))
  (UserInterface|SetWidget _returnvalue_5 _returnvalue_6)
  (Class|WidgetComponent|SetWidgetSpace _returnvalue_5 "Screen")
  (Class|WidgetComponent|SetDrawatDesiredSize _returnvalue_5 true)
  (EventDispatchers|BindEventtoInteractwithBuilding _returnvalue_6 (delegate Custom|BuildingInteract))
  (Variables|Default|SetWidgetComponent _returnvalue_5))

(event EventTick
  (params (DeltaSeconds :type Float%20%28single-precision%29))
  (bind _widgetcomponent (Variables|Default|GetWidgetComponent))
  (Utilities|IsValid (Variables|Default|GetWidgetComponent)
    (:Is%20Valid
      (if (> (Math|Float|NormalizetoRange (Math|Vector|VectorLength (- (Transformation|GetActorLocation (Variables|/Script/Engine.PlayerController|GetPlayerCameraManager (Game|GetPlayerController 0))) (Transformation|GetActorLocation (Components|GetOwner)))) 0.0 5e+03) 1.0)
        (Utilities|FlowControl|Sequence
          (:then_0
            (Utilities|FlowControl|DoOnce false :!label _label
              (:Completed
                (Rendering|SetVisibility _widgetcomponent true false))))
          (:then_1
            (goto _label_2 Reset)))
        (else
          (Utilities|FlowControl|Sequence
            (:then_0
              (Utilities|FlowControl|DoOnce false :!label _label_2
                (:Completed
                  (Rendering|SetVisibility _widgetcomponent false false))))
            (:then_1
              (goto _label Reset))))))))

(event EventSelectBuilding
  (params (bFade? :type Boolean) (CameraSpeed :type Float%20%28double-precision%29) (DisableBorder? :type Boolean))
  (bind _playercharacter (Variables|Default|GetPlayerCharacter))
  (Variables|Default|SetbFade? bFade?)
  (Variables|Default|SetCameraSwitchSpeed CameraSpeed)
  (Variables|Default|SetDisable%20Border? DisableBorder?)
  (Utilities|FlowControl|Delay 0.2)
  (if (not (Variables|/Game/Blueprints/Character/PlayerCamera.PlayerCamera_C|GetTouch _playercharacter))
    (CallFunction|CameratoActionSpots)
    (Variables|/Game/Blueprints/Character/PlayerCamera.PlayerCamera_C|SetInteracted? _playercharacter true)
    (Class|InterfaceActionInteractivewithActor|GetBuildingbyID(Message) (Variables|/Game/Blueprints/Main/MainPlayerController.MainPlayerController_C|GetMainWidget (.AsMain%20Player%20Controller (Utilities|Casting|CastToMainPlayerController (Game|GetPlayerController 0)))) (Variables|Default|GetIndex) (Variables|Default|GetDisable%20Border?) (Components|GetOwner))
    (if (not (Variables|Default|GetbFade?))
      (Default|StopDemonstrationMode (Variables|Default|GetPlayerCharacter)))))

(fn BuildingInteraction
  (params (Enable? :type Boolean))
  (bind _widgetcomponent (Variables|Default|GetWidgetComponent))
  (if Enable?
    (Rendering|SetVisibility _widgetcomponent true false)
    (Variables|Default|SetDisableButton false)
    (else
      (Rendering|SetVisibility _widgetcomponent false false)
      (Variables|Default|SetDisableButton true)))
  (return))