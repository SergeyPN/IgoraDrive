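; MotoRaceInteraction is an interaction actor that launches a moto race along a set of spline actors.
; Enabling it plays each spline's timeline, binds to its race-end event and marks the race as active.
; A counter waits for every spline to finish, then clears the active flag and calls the parent's end event unless it is night.
; Day and night states show or hide the widget only while no race runs.
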(event EventBeginPlay
  (|CallParentFunction) ; This node is disabled and will not be called.\nDrag off pins to build functionality.
)

(event Collision|EventActorBeginOverlap
  (params (OtherActor :type Actor%20Object%20Reference))
  (|CallParentFunction OtherActor) ; This node is disabled and will not be called.\nDrag off pins to build functionality.
)

(event EventTick
  (params (DeltaSeconds :type Float%20%28single-precision%29))
  (|CallParentFunction DeltaSeconds) ; This node is disabled and will not be called.\nDrag off pins to build functionality.
)

(event EventEnableEvent
  (|CallParentFunction)
  (for _array_element (Variables|Default|GetSplines)
    (Default|PlayTimeline _array_element)
    (EventDispatchers|BindEventtoRaceEnd _array_element (EventDispatchers|CreateEvent :!event EventEnd)))
  (Variables|Default|SetAction true))

(event EventEventEnd
  (bind _result (Math|Integer|IncrementInt (Variables|Default|GetMotoCount))
    (:%20%20
      (bind _output_get (Variables|Default|SetMotoCount _result))
      (if (== _output_get (Utilities|Array|Length (Variables|Default|GetSplines)))
        (if (Variables|Default|GetbNight?)
          _
          (else
            (|CallParentFunction)))
        (Variables|Default|SetMotoCount 0)
        (Variables|Default|SetAction false)))))

(event EventDayState
  (|CallParentFunction)
  (if (not (Variables|Default|GetAction))
    (Rendering|SetVisibility (Variables|Default|GetWidget) true false)))

(event EventNightState
  (|CallParentFunction)
  (if (not (Variables|Default|GetAction))
    (Rendering|SetVisibility (Variables|Default|GetWidget) false false)))

(fn ConstructionScript
  (|CallParentFunction))