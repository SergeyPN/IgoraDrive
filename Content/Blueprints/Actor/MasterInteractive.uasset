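; Base actor for interactive objects that show an event button widget, hidden while the event runs or the player camera is far away.
; Tick toggles the widget by camera distance until EnableEvent sets Interacted, and EventEnd restores it.
; BeginPlay hands itself to the button as Owner and binds to UDS sunrise and sunset; DayState and NightState events set a Night flag.
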(event Custom|EnableEvent
  (Variables|Default|SetInteracted true)
  (Rendering|SetVisibility (Variables|Default|GetWidget) false false))

(event Custom|EventEnd
  (Variables|Default|SetInteracted false)
  (Rendering|SetVisibility (Variables|Default|GetWidget) true false))

(event Custom|NightState
  (Variables|Default|SetbNight? true))

(event Custom|DayState
  (Variables|Default|SetbNight? false))

(event EventBeginPlay
  (bind _returnvalue (CallFunction|GetUDS))
  (Variables|Default|SetUDS _returnvalue)
  (bind _asinteractive_event_button (Utilities|Casting|CastToInteractiveEventButton (UserInterface|GetUserWidgetObject (Variables|Default|GetWidget))))
  (Variables|/Game/Blueprints/Widgets/InteractiveEventButton.InteractiveEventButton_C|SetOwner _asinteractive_event_button self)
  (EventDispatchers|BindEventtoSunrise (Variables|Default|GetUDS) (EventDispatchers|CreateEvent :!event Custom|DayState))
  (EventDispatchers|BindEventtoSunset (Variables|Default|GetUDS) (EventDispatchers|CreateEvent :!event Custom|NightState)))

(event EventTick
  (params (DeltaSeconds :type Float%20%28single-precision%29))
  (bind _widget (Variables|Default|GetWidget))
  (if (not (Variables|Default|GetInteracted))
    (if (> (Math|Vector|Distance(Vector) (Transformation|GetActorLocation) (Transformation|GetActorLocation (Variables|/Script/Engine.PlayerController|GetPlayerCameraManager (Game|GetPlayerController 0)))) 2e+04)
      (Rendering|SetVisibility _widget false false)
      (else
        (Rendering|SetVisibility _widget true false)))))

(fn ConstructionScript)