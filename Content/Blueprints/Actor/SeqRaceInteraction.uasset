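; SeqRaceInteraction is an interaction actor that plays a sequence when its event is enabled and is available according to day/night state.
; Enabling plays the sequence player on the Splines reference and sets an Action flag, which the player's OnStop callback clears.
; Day shows and night hides the widget only while no action runs, and the parent's end-of-event logic is skipped at night.
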(event Collision|EventActorBeginOverlap
  (params (OtherActor :type Actor%20Object%20Reference))
  (|CallParentFunction OtherActor) ; This node is disabled and will not be called.\nDrag off pins to build functionality.
)

(event EventTick
  (params (DeltaSeconds :type Float%20%28single-precision%29))
  (|CallParentFunction DeltaSeconds) ; This node is disabled and will not be called.\nDrag off pins to build functionality.
)

(event EventEnableEvent
  (|CallParentFunction)
  (Sequencer|Player|Play (Variables|/Script/LevelSequence.LevelSequenceActor|GetSequencePlayer (Variables|Default|GetSplines)) :!class /Script/MovieScene.MovieSceneSequencePlayer)
  (Variables|Default|SetAction true))

(event EventEventEnd
  (if (Variables|Default|GetbNight?)
    _
    (else
      (|CallParentFunction)))
  (Variables|Default|SetAction false))

(event EventDayState
  (|CallParentFunction)
  (if (not (Variables|Default|GetAction))
    (Rendering|SetVisibility (Variables|Default|GetWidget) true false)))

(event EventNightState
  (|CallParentFunction)
  (if (not (Variables|Default|GetAction))
    (Rendering|SetVisibility (Variables|Default|GetWidget) false false)))

(event EventBeginPlay
  (|CallParentFunction)
  (EventDispatchers|BindEventtoOnStop (Variables|/Script/LevelSequence.LevelSequenceActor|GetSequencePlayer (Variables|Default|GetSplines)) (delegate EventEventEnd)))

(fn ConstructionScript
  (|CallParentFunction))