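; Finish-line actor for AI car races that detects BP_AICar actors through a box overlap.
; Each overlap increments the car's CycleCount; on reaching Count, it calls the car's RaceEnd and stores it in an array.
; When that array add returns index 4 (the fifth finisher), it waits briefly, destroys the stored cars, clears the array and fires InteractionButton's EventEnd.
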(event OnComponentBeginOverlap(Box)
  (params (OverlappedComponent :type Primitive%20Component%20Object%20Reference) (OtherActor :type Actor%20Object%20Reference) (OtherComp :type Primitive%20Component%20Object%20Reference) (OtherBodyIndex :type Integer) (bFromSweep :type Boolean) (SweepResult :type Hit%20Result%20Structure%20%28by%20ref%29))
  (bind _asbp_aicar (Utilities|Casting|CastToBP_AICar OtherActor))
  (bind _result (Math|Integer|IncrementInt (Variables|/Game/Assets/Cars/Chevrolette/BP_AICar.BP_AICar_C|GetCycleCount _asbp_aicar))
    (:%20%20
      (bind _output_get (Variables|/Game/Assets/Cars/Chevrolette/BP_AICar.BP_AICar_C|SetCycleCount _asbp_aicar _result))
      (if (== _output_get (Variables|Default|GetCount))
        (Default|RaceEnd _asbp_aicar)
        (bind _returnvalue (Utilities|Array|Add (Variables|Default|GetAs%20BP%20AICar) _asbp_aicar))
        (if (== _returnvalue 4)
          (Utilities|FlowControl|Delay 3.0)
          (for _array_element (Variables|Default|GetAs%20BP%20AICar)
            (Actor|DestroyActor _array_element))
          (Utilities|Array|Clear (Variables|Default|GetAs%20BP%20AICar))
          (Default|EventEnd (Variables|Default|GetInteractionButton)))))))

(event EventBeginPlay)

(event Collision|EventActorBeginOverlap
  (params (OtherActor :type Actor%20Object%20Reference)))

(event EventTick
  (params (DeltaSeconds :type Float%20%28single-precision%29)))

(fn ConstructionScript)